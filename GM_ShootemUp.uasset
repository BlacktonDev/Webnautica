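; Shoot 'em up game mode that sets the view to BP_Camera and runs data-driven enemy waves.
; Spawn_Loop reads the Enemy_Gameplay_Data row named by a counter and spawns its enemies with per-index health, movement and firing settings.
; It tracks the new spawns, waits the row's duration, then clears them and repeats until no row is found.
; SafeGetArrayElement falls back to the first element for out-of-range indices.
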(event Custom|Spawn_Loop
  (bind _returnvalue (Utilities|GetDataTableRow "/Game/Blueprints/Enemies/Enemy_Gameplay_Data.Enemy_Gameplay_Data" (Utilities|String|StringToName (Utilities|String|ToString(Integer) (Variables|Default|GetSpawn_Loop_Counter))))
    (:then
      (bind _output_get (Variables|Default|SetCurrent_Row_Data _returnvalue))
      (Variables|Default|SetSpawn_Delay (.SeqDuration (Utilities|Struct|BreakST_GameplayStruct _output_get)))
      (Variables|Default|SetScene (.Scene (Utilities|Struct|BreakST_GameplayStruct _output_get)))
      (for _index (range 0 (- (.EnemyCount (Utilities|Struct|BreakST_GameplayStruct _output_get)) 1))
        (Game|SpawnActorfromClass (Utilities|Array|Get(acopy) (Variables|Default|GetEnemy_Classes) (Utilities|SafeGetArrayElement (.Actor (Utilities|Struct|BreakST_GameplayStruct _output_get)) _index)) (Math|Transform|MakeTransform (Utilities|SafeGetArrayElement (.Locations (Utilities|Struct|BreakST_GameplayStruct _output_get)) _index)) "Undefined" "MultiplyWithRoot" 0 (Utilities|SafeGetArrayElement (.Health (Utilities|Struct|BreakST_GameplayStruct _output_get)) _index) 0 (Utilities|SafeGetArrayElement (.Movements (Utilities|Struct|BreakST_GameplayStruct _output_get)) _index) (Utilities|SafeGetArrayElement (.MoveSpeedMulti (Utilities|Struct|BreakST_GameplayStruct _output_get)) _index) (.X (Math|Vector2D|BreakVector2D (Utilities|SafeGetArrayElement (.XYMulti (Utilities|Struct|BreakST_GameplayStruct _output_get)) _index))) (.Y (Math|Vector2D|BreakVector2D (Utilities|SafeGetArrayElement (.XYMulti (Utilities|Struct|BreakST_GameplayStruct _output_get)) _index))) (Utilities|SafeGetArrayElement (.Velocity (Utilities|Struct|BreakST_GameplayStruct _output_get)) _index) (Utilities|SafeGetArrayElement (.CanShoot (Utilities|Struct|BreakST_GameplayStruct _output_get)) _index) (Utilities|SafeGetArrayElement (.FireRate (Utilities|Struct|BreakST_GameplayStruct _output_get)) _index) 0 0)
        (Utilities|Array|AddUnique (Variables|Default|GetEnemies_Just_Spawned) 0))
      (bind _result (Math|Integer|IncrementInt (Variables|Default|GetSpawn_Loop_Counter))
        (:%20%20
          (Variables|Default|SetSpawn_Loop_Counter _result)
          (Utilities|FlowControl|RetriggerableDelay (Variables|Default|GetSpawn_Delay))
          (Utilities|Array|Clear (Variables|Default|GetEnemies_Just_Spawned))
          (CallFunction|SpawnLoop))))))

(event EventBeginPlay
  (bind _returnvalue (Actor|GetActorOfClass "/Game/Blueprints/Character/BP_Camera.BP_Camera_C"))
  (Game|Player|SetViewTargetwithBlend (Game|GetPlayerController 0) _returnvalue 0.0 "VTBlend_Linear" 0.0 false)
  (Utilities|FlowControl|Delay 1.0)
  (CallFunction|SpawnLoop))

(event EventTick
  (params (DeltaSeconds :type Float%20%28single-precision%29)))

(fn ConstructionScript)