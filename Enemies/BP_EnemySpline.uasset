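; Enemy Blueprint that moves its mesh along a spline path at a set speed.
; Each Tick adds speed times delta time to a distance counter, samples the spline's local transform there and applies it as the mesh's relative transform.
; Fixed height and yaw offsets adjust the mesh while its scale is preserved.
; The distance has no wrap, clamp or reversal.
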(event EventBeginPlay
  (|CallParentFunction) ; This node is disabled and will not be called.\nDrag off pins to build functionality.
)

(event Collision|EventActorBeginOverlap
  (params (OtherActor :type Actor%20Object%20Reference))
  (|CallParentFunction OtherActor) ; This node is disabled and will not be called.\nDrag off pins to build functionality.
)

(event EventTick
  (params (DeltaSeconds :type Float%20%28single-precision%29))
  (|CallParentFunction DeltaSeconds)
  (Variables|Default|SetsplineDistance (+ (* DeltaSeconds (Variables|Default|GetsplineSpeed)) (Variables|Default|GetsplineDistance)))
  (Transformation|SetRelativeTransform (Variables|Character|GetMesh) (Math|Transform|MakeTransform (Math|Vector|MakeVector (.x (.location (Spline|GetTransformatDistanceAlongSpline (Variables|Default|GetSpline) (Variables|Default|GetsplineDistance) "Local" false))) (.y (.location (Spline|GetTransformatDistanceAlongSpline (Variables|Default|GetSpline) (Variables|Default|GetsplineDistance) "Local" false))) (+ (.z (.location (Spline|GetTransformatDistanceAlongSpline (Variables|Default|GetSpline) (Variables|Default|GetsplineDistance) "Local" false))) -89.0)) (Math|Rotator|MakeRotator (.roll (.rotation (Spline|GetTransformatDistanceAlongSpline (Variables|Default|GetSpline) (Variables|Default|GetsplineDistance) "Local" false))) (.pitch (.rotation (Spline|GetTransformatDistanceAlongSpline (Variables|Default|GetSpline) (Variables|Default|GetsplineDistance) "Local" false))) (+ (.yaw (.rotation (Spline|GetTransformatDistanceAlongSpline (Variables|Default|GetSpline) (Variables|Default|GetsplineDistance) "Local" false))) -9e+01)) (Variables|/Script/Engine.SceneComponent|GetRelativeScale3D (Variables|Character|GetMesh))) false false))

(fn ConstructionScript
  (|CallParentFunction))