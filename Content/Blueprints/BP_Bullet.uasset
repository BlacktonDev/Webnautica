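; Bullet projectile actor with an active/inactive flag, moved by physics force on its Sphere component.
; Shoot stores the damage and pushes the sphere along the given direction scaled by Force; the SpeedMultiplier input is unused.
; Active and Deactive set IsActive and both call Activate on the root; only Deactive changes visibility, hiding the sphere.
; No overlap or hit logic applies the stored damage here.
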(event EventBeginPlay)

(event Collision|EventActorBeginOverlap
  (params (OtherActor :type Actor%20Object%20Reference)))

(event EventTick
  (params (DeltaSeconds :type Float%20%28single-precision%29)))

(fn ConstructionScript)

(fn Shoot
  (params (Direcction :type Vector) (SpeedMultiplier :type Float%20%28double-precision%29) (Damage :type Float%20%28double-precision%29))
  ;[0.5781 0 0.5716] Funcion de disparo de bala
  (Variables|Default|SetDamage Damage)
  (Physics|AddForce (Variables|Default|GetSphere) (* Direcction (Variables|Default|GetForce)) "None" false))

(fn Active
  (Components|Activation|Activate (Variables|Default|GetDefaultSceneRoot) false)
  (Variables|Default|SetisActive true))

(fn Deactive
  (Components|Activation|Activate (Variables|Default|GetDefaultSceneRoot) false)
  (Variables|Default|SetisActive false)
  (Rendering|SetVisibility (Variables|Default|GetSphere) false false))