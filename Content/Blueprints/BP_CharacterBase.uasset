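; BP_CharacterBase is a player character that moves with Enhanced Input and fires bullets from two alternating cannons.
; BeginPlay adds the character's mapping context, and the movement action drives world-axis movement with Y inverted.
; Firing spawns BP_Bullet at the current cannon and shoots it along the capsule's forward vector, with speed multiplier and damage passed as zero.
; A FlipFlop toggles the cannon after each shot, and a delay gates the fire cooldown.
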(event Input|EnhancedActionEvents|EnhancedInputActionIA_Movimiento
  (params (ActionValue :type Vector%202D%20Structure) (ElapsedSeconds :type Float%20%28double-precision%29) (TriggeredSeconds :type Float%20%28double-precision%29) (InputAction :type Input%20Action%20Object%20Reference :default "/Game/Input/IA_Movimiento.IA_Movimiento"))
  (bind (_x _y) (Math|Vector2D|BreakVector2D ActionValue))
  (:Triggered
    (Pawn|Input|AddMovementInput (Math|Vector|MakeVector _x (* _y -1.0) 0.0) 1.0 false)))

(event Input|EnhancedActionEvents|EnhancedInputActionIA_Fire
  (params (ActionValue :type Boolean) (ElapsedSeconds :type Float%20%28double-precision%29) (TriggeredSeconds :type Float%20%28double-precision%29) (InputAction :type Input%20Action%20Object%20Reference :default "/Game/Input/IA_Fire.IA_Fire"))
  (:Triggered
    (if (Variables|Default|GetcanFire)
      (bind _returnvalue (Game|SpawnActorfromClass "/Game/Blueprints/BP_Bullet.BP_Bullet_C" (Transformation|GetWorldTransform (select (Variables|Default|GetisCanon) (Variables|Default|GetCanon2) (Variables|Default|GetCanon1))) "Undefined" "MultiplyWithRoot" 0 0))
      (Default|Shoot _returnvalue (Math|Vector|GetForwardVector (Variables|Collision|GetCapsuleComponent)) 0.0 0.0)
      (bind _isa (Utilities|FlowControl|FlipFlop)
        (:A
          _)
        (:B
          _))
      (Variables|Default|SetisCanon _isa)
      (Variables|Default|SetcanFire false)
      (Utilities|FlowControl|Delay (Variables|Default|GetfireCooldown))
      (Variables|Default|SetcanFire true))))

(event EventBeginPlay
  (Input|AddMappingContext (PlayerController|LocalPlayerSubsystems|GetEnhancedInputLocalPlayerSubsystem (Game|GetPlayerController 0)) "/Game/Input/IMC_CharacterBase.IMC_CharacterBase" 0 "(bIgnoreAllPressedKeysUntilRelease=True,bForceImmediately=False)"))

(fn ConstructionScript)