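; Bullet pool owned by a BP_CharacterBase, meant to pre-spawn and recycle BP_Bullet actors.
; On BeginPlay it spawns bullets, counted by AmountOfBullets, at one of two cannon transforms chosen by IsCanon and disables their mesh collision.
; A return event moves a bullet to the owner and attaches it.
; The nodes that attach new bullets, bind that event and fill BulletsPool are disconnected, so pooling is incomplete.
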(event Custom|RetrurnToPool
  (params (Bullet :type BP%20Bullet%20Object%20Reference))
  (bind _returnvalue (Components|GetOwner))
  (Transformation|SetActorLocation Bullet (Transformation|GetActorLocation _returnvalue) false false)
  (Transformation|AttachActorToActor Bullet _returnvalue "None" "KeepWorld" "KeepWorld" "KeepWorld" true))

(event EventBeginPlay
  (bind _asbp_character_base (Utilities|Casting|CastToBP_CharacterBase (Components|GetOwner)))
  (for _index (range 0 (Variables|Default|GetAmountOfBullets))
    (bind _returnvalue (Game|SpawnActorfromClass "/Game/Blueprints/Projectiles/BP_Bullet.BP_Bullet_C" (Transformation|GetWorldTransform (select (Variables|/Game/Blueprints/Character/BP_CharacterBase.BP_CharacterBase_C|GetisCanon _asbp_character_base) (Variables|/Game/Blueprints/Character/BP_CharacterBase.BP_CharacterBase_C|GetCanon2 _asbp_character_base) (Variables|/Game/Blueprints/Character/BP_CharacterBase.BP_CharacterBase_C|GetCanon1 _asbp_character_base))) "Undefined" "MultiplyWithRoot" 0 0))
    (Collision|SetCollisionEnabled (Variables|/Game/Blueprints/Projectiles/BP_Bullet.BP_Bullet_C|GetBulletMesh _returnvalue) "NoCollision")))

(event EventTick
  (params (DeltaSeconds :type Float%20%28single-precision%29)))