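; BP_CharacterBase is a player character with Enhanced Input movement and firing from a bullet pool.
; IA_Fire calls Shoot along the capsule's forward vector on the BP_Bullet found by GetActorOfClass, then detaches the indexed pool bullet and increments the index.
; Setup caches both cannon positions.
; Fire-rate cooldown, cannon alternation and index wraparound logic exist but are unconnected.
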(event Custom|Setup
  (Variables|Default|Setcanon1Pos (Transformation|GetWorldLocation (Variables|Default|GetCanon1)))
  (Variables|Default|Setcanon2Pos (Transformation|GetWorldLocation (Variables|Default|GetCanon2))))

(event Input|EnhancedActionEvents|EnhancedInputActionIA_Movimiento
  (params (ActionValue :type Vector%202D%20Structure) (ElapsedSeconds :type Float%20%28double-precision%29) (TriggeredSeconds :type Float%20%28double-precision%29) (InputAction :type Input%20Action%20Object%20Reference :default "/Game/Input/IA_Movimiento.IA_Movimiento"))
  (bind (_x _y) (Math|Vector2D|BreakVector2D ActionValue))
  ;[0 0.2367 1] Movimiento
  (:Triggered
    (Pawn|Input|AddMovementInput (Math|Vector|MakeVector _x (* _y -1.0) 0.0) 1.0 false)))

(event Input|EnhancedActionEvents|EnhancedInputActionIA_Fire
  (params (ActionValue :type Boolean) (ElapsedSeconds :type Float%20%28double-precision%29) (TriggeredSeconds :type Float%20%28double-precision%29) (InputAction :type Input%20Action%20Object%20Reference :default "/Game/Input/IA_Fire.IA_Fire"))
  (bind _bp_bulletpool (Variables|Default|GetBP_BulletPool))
  (bind _bulletspool (Variables|/Game/Blueprints/Character/BP_BulletPool.BP_BulletPool_C|GetBulletsPool _bp_bulletpool))
  (bind _returnvalue (Utilities|Array|Length _bulletspool))
  ;[1 0.4122 0] Disparo
  (:Triggered
    (if (> _returnvalue 0)
      (Variables|Default|SetMaxPool _returnvalue)
      (Utilities|IsValid (Utilities|Array|Get(acopy) _bulletspool (Variables|Default|GetBulletIndex))
        (:Is%20Valid
          (if (Variables|Default|GetcanFire)
            (bind _returnvalue_2 (Actor|GetActorOfClass "/Game/Blueprints/Projectiles/BP_Bullet.BP_Bullet_C"))
            (Default|Shoot _returnvalue_2 (Math|Vector|GetForwardVector (Variables|Collision|GetCapsuleComponent)) 0.0 0.0)
            (Transformation|DetachFromActor (Utilities|Array|Get(acopy) _bulletspool (Variables|Default|GetBulletIndex)) "KeepWorld" "KeepWorld" "KeepWorld")
            (bind _result (Math|Integer|IncrementInt (Variables|Default|GetBulletIndex))
              (:%20%20
                (bind _output_get (Variables|Default|SetBulletIndex _result))))))))))

(event EventBeginPlay
  ;[0 0.2367 1] Movimiento
  (Input|AddMappingContext (PlayerController|LocalPlayerSubsystems|GetEnhancedInputLocalPlayerSubsystem (Game|GetPlayerController 0)) "/Game/Input/IMC_CharacterBase.IMC_CharacterBase" 0 "(bIgnoreAllPressedKeysUntilRelease=True,bForceImmediately=False)"))

(fn ConstructionScript)