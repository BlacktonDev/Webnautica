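; BP_Bullet is a physics-driven projectile that destroys itself and fires its OnBulletDestroy dispatcher on overlapping an actor tagged Wall.
; Shoot stores Damage and pushes the mesh with a force along the given direction, leaving SpeedMultiplier unused.
; Active and Deactive toggle the active flag and physics simulation, as if for reuse, but both hide the mesh.
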(event EventBeginPlay)

(event Collision|EventActorBeginOverlap
  (params (OtherActor :type Actor%20Object%20Reference))
  (if (Actor|ActorHasTag OtherActor "Wall")
    (Actor|DestroyActor)
    (Default|CallOnBulletDestroy self)))

(event EventTick
  (params (DeltaSeconds :type Float%20%28single-precision%29)))

(fn ConstructionScript)

(fn Shoot
  (params (Direcction :type Vector) (SpeedMultiplier :type Float%20%28double-precision%29) (Damage :type Float%20%28double-precision%29))
  ;[0.5781 0 0.5716] Funcion de disparo de bala
  (Variables|Default|SetDamage Damage)
  (Physics|AddForce (Variables|Default|GetBulletMesh) (* Direcction (Variables|Default|GetForce)) "None" false))

(fn Active
  (Components|Activation|Activate (Variables|Default|GetDefaultSceneRoot) false)
  (Variables|Default|SetisActive true)
  (Rendering|SetVisibility (Variables|Default|GetBulletMesh) false false)
  (Physics|SetSimulatePhysics (Variables|Default|GetBulletMesh) true))

(fn Deactive
  (Components|Activation|Activate (Variables|Default|GetDefaultSceneRoot) false)
  (Variables|Default|SetisActive false)
  (Rendering|SetVisibility (Variables|Default|GetBulletMesh) false false)
  (Physics|SetSimulatePhysics (Variables|Default|GetBulletMesh) false))